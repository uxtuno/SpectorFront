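; Game mode that ends a stage when its level sequence finishes and shows the stage clear screen.
; On BeginPlay and after each level transition, it caches the unique LevelSequenceActor and opens a gate that Tick feeds to poll playback position.
; At the sequence's end it pauses, displays WBP_StageClear, stores score and player HP plus a bonus in BP_GameInstance for the next stage, then closes the gate.
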(event `PostLevelTransition`
  (bind _returnvalue (`MyBlueprintFunctionLibrary.FindUniqueActorOfClass` "/Game/BluePrints/Player/BP_PlayerController.BP_PlayerController_C"))
  (bind (_uniqueactor _success) (`/Game/BluePrints/MyLibrary/MyLib.GetUniqueActorOfClass` "/Script/LevelSequence.LevelSequenceActor"))
  (bind _sequencer (`self.Sequencer`))
  (bind _asbp_game_instance (cast `/Game/BluePrints/BP_GameInstance` (`GameplayStatics.GetGameInstance`) :!pure true))
  (bind _sequenceplayer (`LevelSequenceActor.SequencePlayer` _sequencer))
  (bind _returnvalue_2 (`GameplayStatics.GetCurrentLevelName` true :!label _label))
  (`KismetSystemLibrary.PrintString` _returnvalue_2)
  (if _success
    (bind _aslevel_sequence_actor (cast `LevelSequenceActor` _uniqueactor))
    (set `self.Sequencer` _aslevel_sequence_actor)
    (goto _label_2 :!via `Open`)))

(event `self.ReceiveBeginPlay`
  (bind _asbp_game_instance (cast `/Game/BluePrints/BP_GameInstance` (`GameplayStatics.GetGameInstance`)))
  (add `/Game/BluePrints/BP_GameInstance.PostLevelTransitionDelegate` _asbp_game_instance (delegate `PostLevelTransition`))
  (goto _label))

(event `self.ReceiveTick`
  (params (DeltaSeconds :type "Float (single-precision)"))
  (bind _returnvalue (`MyBlueprintFunctionLibrary.FindUniqueActorOfClass` "/Game/BluePrints/Player/BP_PlayerController.BP_PlayerController_C"))
  (bind _sequencer (`self.Sequencer`))
  (bind _asbp_game_instance (cast `/Game/BluePrints/BP_GameInstance` (`GameplayStatics.GetGameInstance`) :!pure true))
  (bind _sequenceplayer (`LevelSequenceActor.SequencePlayer` _sequencer))
  ;[1 1 1] シーケンサー終了で自動遷移
  (`/Engine/EditorBlueprintResources/StandardMacros.Gate` true :!label _label_2
    (:`Exit`
      (`/Engine/EditorBlueprintResources/StandardMacros.IsValid` _sequencer
        (:`Is Valid`
          (if (>= (`LevelSequencePlayer.GetPlaybackPosition` _sequenceplayer) (`LevelSequencePlayer.GetLength` _sequenceplayer))
            (`GameplayStatics.SetGamePaused` true)
            (bind _returnvalue_2 (`|CreateWidget` "/Game/BluePrints/UI/WBP_StageClear.WBP_StageClear_C"))
            (`/Engine/EditorBlueprintResources/StandardMacros.IsValid` _returnvalue
              (:`Is Valid`
                (`WidgetBlueprintLibrary.SetInputMode_GameAndUIEx` _returnvalue _returnvalue_2 true)
                (`UserWidget.AddToViewport` _returnvalue_2 0)
                ;[1 1 1] ステージ間の引き継ぎ処理
                (`/Game/BluePrints/BP_GameInstance.SetTakeOverScore` _asbp_game_instance (`/Game/BluePrints/BP_GameState.GetScore` (cast `/Game/BluePrints/BP_GameState` (`GameplayStatics.GetGameState`) :!pure true)))
                (`/Game/BluePrints/BP_GameInstance.SetTakeOverHP` _asbp_game_instance (+ (`PlayerCharacter.hp` (cast `/Game/BluePrints/Player/BP_Player` (`GameplayStatics.GetPlayerCharacter` 0) :!pure true)) (`self.NextStageToAddHP`)))
                (goto _label_2 :!via `Close`)))))))))

(fn `UserConstructionScript`)