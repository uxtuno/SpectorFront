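; Player controller Blueprint that sets up the reticle HUD and handles the player's game over.
; On BeginPlay it adds a reticle widget to the viewport and binds to the HP change dispatcher on BP_Player.
; When HP drops to zero or below, it pauses the level sequence and the game, then shows a game over widget with game-and-UI input focused on it.
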(event `self.ReceiveBeginPlay`
  (add `/Game/BluePrints/Player/BP_Player.HpChangeDispatcher` (`MyBlueprintFunctionLibrary.FindUniqueActorOfClass` "/Game/BluePrints/Player/BP_Player.BP_Player_C") (delegate `OnPlayerHpChanged`))
  (bind _returnvalue (`|CreateWidget` "/Game/BluePrints/UI/WBP_Reticle.WBP_Reticle_C" self))
  (`UserWidget.AddToViewport` _returnvalue 10))

(event `OnPlayerHpChanged`
  (params (NewHp :type "Float (double-precision)"))
  (if (<= NewHp 0.0)
    (`LevelSequencePlayer.Pause` (`LevelSequenceActor.SequencePlayer` (`MyBlueprintFunctionLibrary.FindUniqueActorOfClass` "/Script/LevelSequence.LevelSequenceActor")))
    (`GameplayStatics.SetGamePaused` true)
    (bind _returnvalue (`|CreateWidget` "/Game/BluePrints/UI/WBP_GameOver.WBP_GameOver_C"))
    (`WidgetBlueprintLibrary.SetInputMode_GameAndUIEx` self _returnvalue false false)
    (`UserWidget.AddToViewport` _returnvalue 0)))

(fn `UserConstructionScript`)