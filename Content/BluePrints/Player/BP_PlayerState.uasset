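; BP_PlayerState is the player state that stores the player's score and provides functions to get, set and add to it.
; AddScore routes through SetScore, which stores the value, fires the ScoreChange dispatcher to notify listeners and returns the score.
; On BeginPlay it also caches a reference to the unique BP_Player actor, which the score functions do not use.
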(event `self.ReceiveBeginPlay`
  (set `self.Player` (`MyBlueprintFunctionLibrary.FindUniqueActorOfClass` "/Game/BluePrints/BP_Player.BP_Player_C")))

(fn `AddScore`
  (params (PlayerScore :type Integer))
  (returns (NewScore :type Integer))
  (bind _newscore (`self.SetScore` (+ PlayerScore (`self.PlayerScore`))))
  (return _newscore))

(fn `GetScore`
  (returns (PlayerScore :type Integer))
  (return (`self.PlayerScore`)))

(fn `SetScore`
  (params (PlayerScore :type Integer))
  (returns (NewScore :type Integer))
  (bind _output_get (set `self.PlayerScore` PlayerScore))
  (`self.ScoreChangeDispatcher` _output_get)
  (return _output_get))

(fn `UserConstructionScript`)