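; BP_PlayerCamera is a player camera actor, with its only placement logic in the Construction Script.
; On construction, it traces downward on the Visibility channel and snaps itself to a fixed height above the surface it hits.
; At runtime it only prints a debug string on BeginPlay.
; An unconnected node that zeroes BP_Player's Hp never runs.
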(event `self.ReceiveBeginPlay`
  (`KismetSystemLibrary.PrintString` "Camera"))

(fn `UserConstructionScript`
  (bind _returnvalue (`self.K2_GetActorLocation`))
  (bind (_outhit _returnvalue_2) (`KismetSystemLibrary.LineTraceSingle` _returnvalue (+ _returnvalue (0.0 0.0 -1000.0)) "TraceTypeQuery1"))
  (if _returnvalue_2
    (`self.K2_SetActorLocation` (+ (`.ImpactPoint` (`GameplayStatics.BreakHitResult` _outhit)) (0.0 0.0 150.0)))))