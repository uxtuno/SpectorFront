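; BP_Player is the player Blueprint, holding hit points and riding on the player camera actor.
; On BeginPlay it finds the unique BP_PlayerCamera, caches its camera and snaps itself onto that actor.
; Only when the camera exists does it also subscribe to the game state's score observable, printing each new score.
; Damage events subtract from Hp and broadcast the new value through a change dispatcher.
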(event `self.ReceiveBeginPlay`
  (bind _returnvalue (`MyBlueprintFunctionLibrary.FindUniqueActorOfClass` "/Game/BluePrints/Player/BP_PlayerCamera.BP_PlayerCamera_C"))
  (`/Engine/EditorBlueprintResources/StandardMacros.IsValid` _returnvalue
    (:`Is Valid`
      (set `self.PlayerCamera` (`/Game/BluePrints/Player/BP_PlayerCamera.Camera` _returnvalue))
      (`self.K2_AttachToActor` _returnvalue "None" "SnapToTarget" "SnapToTarget" "SnapToTarget" false)
      (add `/Game/BluePrints/BP_GameState.ScoreObservable` (cast `/Game/BluePrints/BP_GameState` (`GameplayStatics.GetGameState`) :!pure true) (delegate `OnScoreChanged`)))))

(event `OnScoreChanged`
  (params (NewScore :type Integer))
  (`KismetSystemLibrary.PrintString` (`KismetStringLibrary.Conv_IntToString` NewScore)))

(event `self.OnDamage`
  (params (damage :type "Float (single-precision)") (instigatedBy :type "Controller Object Reference") (damageCauser :type "Actor Object Reference"))
  (bind _output_get (set `self.hp` (- (`self.hp`) damage)))
  (`self.HpChangeDispatcher` _output_get))

(fn `UserConstructionScript`)