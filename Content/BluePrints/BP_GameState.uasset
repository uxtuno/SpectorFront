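; BP_GameState is a game state Blueprint that holds the game's score and announces its changes.
; SetScore stores the value, fires the ScoreObservable dispatcher with it and returns it, giving listeners an observer-style update.
; AddScore computes a sum and routes it through SetScore, so additions also broadcast, while GetScore returns the stored score.
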(fn `AddScore`
  (params (score :type Integer))
  (returns (newScore :type Integer))
  (bind _newscore (`self.SetScore` (+ score (`self.Score`))))
  (return _newscore))

(fn `GetScore`
  (returns (newScore :type Integer))
  (return (`self.Score`)))

(fn `SetScore`
  (params (score :type Integer))
  (returns (newScore :type Integer))
  (bind _output_get (set `self.Score` score))
  (`self.ScoreObservable` _output_get)
  (return _output_get))

(fn `UserConstructionScript`)