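; BP_EnemySpawner spawns enemies in the game flow and decides when its spawn phase is finished.
; BeginSpawn spawns at a zero relative offset, then calls EndSpawn.
; While spawning, Tick calls Finish directly if annihilation finish is enabled, no spawned enemies remain and generation is done.
; Otherwise, chained Delays force Finish after a timeout plus a surplus wait; derived Tick overrides are expected to call the parent.
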(event `self.BeginSpawn`
  ;[1 0.8973 0.1375] 生成処理
  (`self.EnemySpawnRelative` (0.0 0.0 0.0))
  (`self.EndSpawn`))

(event `self.ReceiveTick`
  (params (DeltaSeconds :type "Float (single-precision)"))
  ;[1 1 1] 終了判定
  (`parent.ReceiveTick` DeltaSeconds)
  (if (`self.isSpawning`)
    (if (not (and (== (`self.GetSpawnedEnemyCount`) 0) (`self.IsAnnihilationFinish`) (not (`self.isGenerating`))))
      (`KismetSystemLibrary.Delay` (`self.ForceFinishSeonds`)) ; 一定時間待機で強制的に終了させる
      (`KismetSystemLibrary.Delay` (`self.SurplusWaitSeconds`)) ; 終了後の待機時間
    )
    ;;[1 1 1] 制御終了
    (`self.Finish`)))

(fn `UserConstructionScript`)