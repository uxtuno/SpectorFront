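; BP_RandomSpawner repeatedly spawns enemies at random positions within a radius around itself.
; BeginSpawn selects GroundSpawn, which uses random flat offsets for relative spawning, or SphereSpawn, which picks navigable NavMesh points.
; Both loop on a delay, with a DoOnce passing execution out after the first spawn.
; Only SphereSpawn checks IsSpawning to stop looping.
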(event `self.BeginSpawn`
  ;[1 0.7707 0.1674] 生成
  (if (`self.IsGroundSpawn`)
    (`self.GroundSpawn`)
    (else
      (`self.SphereSpawn`))))

(fn `UserConstructionScript`)