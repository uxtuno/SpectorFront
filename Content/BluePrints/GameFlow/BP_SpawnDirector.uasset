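; BP_SpawnDirector controls an enemy spawn sequence, delaying the parent's spawn trigger and deciding when it finishes.
; It finishes when its SeeTargetFinish enemy dies or that target spawner starts spawning.
; Otherwise, Tick ends non-endless spawns through Delays: a force-finish timeout, skipped on annihilation when enabled, then a late wait.
; AllKill kills spawned enemies, and the construction script's child-actor centering is disconnected.
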(event Custom|notifiEnemyDieEventDispather_Event_0
  (params (enemy :type Enemy%20Interface%20Interface))
  ;[1 1 1] 設定した対象がエネミーならその敵が死んだときに終了
  (Class|AbstractEnemySpawner|Finish))

(event EventBeginPlay
  ;[1 1 1] 設定した対象がエネミーならその敵が死んだときに終了
  (|CallParentFunction)
  (bind _asbp_base_enemy (Utilities|Casting|CastToBP_BaseEnemy (Variables|Default|GetseeTargetFinish)))
  (EventDispatchers|AssignNotifiEnemyDieEventDispather _asbp_base_enemy (delegate Custom|notifiEnemyDieEventDispather_Event_0)))

(event EventTriggerSpawn
  (params (parent :type Abstract%20Enemy%20Spawner%20Object%20Reference) (callback :type Finish%20Spawn%20Structure) (allEnemies :type Actor%20Container%20Object%20Reference))
  ;[1 1 1] 起動遅延
  (Utilities|FlowControl|Delay (Variables|EnemySpawner|GetStartDelaySeconds))
  (|CallParentFunction parent callback allEnemies))

(event EventTick
  (params (DeltaSeconds :type Float%20%28single-precision%29))
  ;[1 1 1] 終了判定
  (|CallParentFunction DeltaSeconds)
  (bind _asabstract_enemy_spawner (Utilities|Casting|CastToAbstractEnemySpawner (Variables|Default|GetseeTargetFinish))
    (:then
      (if (Variables|/Script/SpecterFront.AbstractEnemySpawner|GetisSpawning _asabstract_enemy_spawner)
        ;[1 1 1] 終了
        (Class|AbstractEnemySpawner|Finish)
        (else
          (if (not (Variables|EnemySpawner|GetIsEndless)) :!label _label
            (if (Variables|Default|GetisSpawning)
              (if (Math|Boolean|ANDBoolean (== (Class|AbstractEnemySpawner|GetSpawnedEnemyCount) 0) (Variables|Default|GetIsAnnihilationFinish) (not (Variables|Default|GetisGenerating)))
                _
                (else
                  (Utilities|FlowControl|Delay (Variables|EnemySpawner|GetForceFinishSeonds)) ; 一定時間待機で強制的に終了させる
                ))
              (Utilities|FlowControl|Delay (Variables|EnemySpawner|GetLateWaitSeconds)) ; 終了後の待機時間
              ;;[1 1 1] 制御終了
              (Class|AbstractEnemySpawner|Finish))))))
    (:CastFailed
      (goto _label))))

(fn ConstructionScript)

(fn AllKill
  (for _array_element (Variables|Default|GetspawnedEnemies)
    (bind _asbase_enemy (Utilities|Casting|CastToBaseEnemy _array_element))
    (Class|BaseEnemy|Kill _asbase_enemy))
  (return))