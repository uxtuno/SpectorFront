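; A game-flow spawn director that triggers a list of spawners one after another at a timed interval.
; BeginSpawn walks Spawners with a continue-driven loop, calling TriggerSpawn with itself and AllEnemies, then delaying IntervalSeconds before the next.
; After each full pass it restarts endlessly if Repeate is negative, otherwise it increments RepeateCount and calls EndSpawn once that reaches the limit.
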(event `self.Initialize`
  ;[1 1 1] 初期化
  (set `self.RepeateCount` 0))

(event `self.BeginSpawn`
  (bind _element (`/Game/BluePrints/MyLibrary/MyLoopMacros.ForeachLoopWithContinue` (`self.spawners`) :!label _label)
    (:`LoopBody`
      (`self.TriggerSpawn` :`self` _element :`parent` self :`allEnemies` (`self.allEnemies`))
      (`KismetSystemLibrary.Delay` (`self.IntervalSeconds`))
      (goto _label :!via `Continue`))
    (:`Complete`
      (if (< (`self.Repeate`) 0)
        (goto _label)
        (else
          (bind _result (`/Engine/EditorBlueprintResources/StandardMacros.IncrementInt` (`self.RepeateCount`))
            (:`  `
              (if (>= _result (`self.Repeate`))
                (`self.EndSpawn`)
                (else
                  (goto _label))))))))))

(event `self.ReceiveTick`
  (params (DeltaSeconds :type "Float (single-precision)"))
  (`parent.ReceiveTick` DeltaSeconds))

(fn `UserConstructionScript`
  (`parent.UserConstructionScript`))