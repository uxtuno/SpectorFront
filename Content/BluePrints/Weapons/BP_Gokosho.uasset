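; BP_Gokosho is a weapon actor that flies along its local move direction and later homes in on the player character.
; A timeline, played from Tick, scales travel speed over time and fires an event track that switches on following.
; While following, each timeline update lerps rotation by a fixed alpha toward a point offset from the player, curving the local-space movement.
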(event `self.ReceiveBeginPlay`
  (set `self.Player` (`MyBlueprintFunctionLibrary.FindUniqueActorOfClass` "/Script/SpecterFront.PlayerCharacter")))

(event `self.ReceiveTick`
  (params (DeltaSeconds :type "Float (single-precision)"))
  (bind (_direction _speed) (`Timeline|SpeedTimeLine`)
    (:`Update`
      (`|ExecutionSequence`
        (:`then_0`
          (`self.K2_AddActorLocalOffset` (* (`self.MoveDirection`) (* _speed DeltaSeconds (`self.Speed`)))))
        (:`then_1`
          (if (`self.IsPlayerFollowing`)
            (`self.K2_SetActorRotation` (`KismetMathLibrary.RLerp` (`self.K2_GetActorRotation`) (`KismetMathLibrary.FindLookAtRotation` (`self.K2_GetActorLocation`) (+ (`self.K2_GetActorLocation` (`self.Player`)) (100.0 0.0 80.0))) 0.05 true))))))
    (:`PlayerForrowing`
      (set `self.IsPlayerFollowing` true))))

(fn `UserConstructionScript`)