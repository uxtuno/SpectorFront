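; Actor component that makes its owning actor float up and down along Z.
; BeginPlay randomizes the phase T and the amplitude Width, so instances move differently.
; Each Tick adds a sine offset from T and Width to the owner's current location without sweep, so it accumulates frame by frame.
; T advances by delta time divided by Seconds and wraps past two pi.
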(event EventBeginPlay
  (Variables|Default|Sett (Math|Random|RandomFloat))
  (Variables|Default|SetWidth (Math|Random|RandomFloat)))

(event EventTick
  (params (DeltaSeconds :type Float%20%28single-precision%29))
  (bind _returnvalue (Components|GetOwner))
  (bind _returnvalue_2 (|(2*(PI()))))
  (Utilities|FlowControl|Sequence
    (:then_0
      (Transformation|SetActorLocation _returnvalue (+ (Transformation|GetActorLocation _returnvalue) (Math|Vector|MakeVector 0.0 0.0 (|((sin((({5CD4C653-4752-1CA5-09F6-47BFCD8ECE6E}*2)*(pi()))))*{C28B684E-4D6E-666A-5205-529410C3D1A4})))) false false))
    (:then_1
      (bind _output_get (Variables|Default|Sett (+ (/ DeltaSeconds (Variables|Default|GetSeconds)) (Variables|Default|Gett))))
      (if (> _output_get _returnvalue_2)
        (Variables|Default|Sett (- (Variables|Default|Gett) _returnvalue_2))))))