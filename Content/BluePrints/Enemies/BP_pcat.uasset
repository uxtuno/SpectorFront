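; BP_pcat is an enemy that chases the player and dies on contact with it.
; Attack turns it to face the player pawn and has its AI controller move toward that pawn, stopping within an acceptance radius.
; Overlapping an actor tagged Player calls Kill and destroys the enemy.
; BeginPlay records the start location, which this file never reads, and a manual speed-based movement calculation is left unused.
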(event `self.ReceiveBeginPlay`
  (set `self.StartLocation` (`self.K2_GetActorLocation`)))

(event `self.ReceiveActorBeginOverlap`
  (params (OtherActor :type "Actor Object Reference"))
  ;[1 1 1] プレイヤーにぶつかれば死ぬ
  (if (`self.ActorHasTag` OtherActor "Player")
    (`self.Kill` null)
    (`self.K2_DestroyActor`)))

(fn `Attack`
  (params (deltaTime :type "Float (double-precision)"))
  (`self.K2_SetActorRotation` (`KismetMathLibrary.FindLookAtRotation` (`self.K2_GetActorLocation`) (`self.K2_GetActorLocation` (`GameplayStatics.GetPlayerPawn` 0))))
  (`AIController.MoveToActor` (cast `AIController` (`self.GetController`) :!pure true) (`GameplayStatics.GetPlayerPawn` 0) 500.0 true true true null true))

(fn `UserConstructionScript`
  (`parent.UserConstructionScript`))