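; BP_kuri is an enemy that spins its skeletal mesh while shifting back and forth, and can pursue the player.
; Every Tick it adds a fixed rotation and uses a wrapping frame counter to alternate between two swept location offsets, independent of delta time.
; Its Attack function turns the actor toward player pawn 0 and has the AI controller move to that pawn with a wide acceptance radius.
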(event `self.ReceiveTick`
  (params (DeltaSeconds :type "Float (single-precision)"))
  (`SceneComponent.K2_AddWorldRotation` (`self.SkeletalMesh`) (struct :`Yaw` 5.0) false false)
  (if (> (`self.NewVar_0`) 0)
    (`self.K2_SetActorLocation` (+ (`self.K2_GetActorLocation`) (`self.NewVar_2`)) true)
    (else
      (`self.K2_SetActorLocation` (+ (`self.K2_GetActorLocation`) (`self.NewVar_1`)) true)))
  (if (> (`self.NewVar_0`) 29)
    (set `self.NewVar_0` -30)
    (else
      (`/Engine/EditorBlueprintResources/StandardMacros.IncrementInt` (`self.NewVar_0`)))))

(fn `Attack`
  (params (deltaTime :type "Float (double-precision)"))
  (`self.K2_SetActorRotation` (`KismetMathLibrary.FindLookAtRotation` (`self.K2_GetActorLocation`) (`self.K2_GetActorLocation` (`GameplayStatics.GetPlayerPawn` 0))))
  (`AIController.MoveToActor` (cast `AIController` (`self.GetController`) :!pure true) (`GameplayStatics.GetPlayerPawn` 0) 500.0 true true true null true))

(fn `UserConstructionScript`
  (`parent.UserConstructionScript`))