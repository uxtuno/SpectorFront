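; Spawner Blueprint that repeatedly spawns enemies at random positions within a radius, using a parent class's spawn functions.
; IsGroundSpawn selects either flat random offsets relative to the spawner or random navigable NavMesh points, each looped through a Delay.
; Finish logic skips the forced timeout if IsSpawning, no enemies remain and annihilation finish is enabled, then waits a surplus delay before calling FinishSpawn.
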(event `OnBeginSpawn`
  (`|ExecutionSequence`
    (:`then_0`
      (if (`self.IsGroundSpawn`)
        (`self.GroundSpawn`)
        (else
          (`self.SphereSpawn`))))
    (:`then_1`
      (goto _label :!via `Reset`))))

(event `self.ReceiveTick`
  (params (DeltaSeconds :type "Float (single-precision)"))
  (`parent.ReceiveTick` DeltaSeconds)
  (`/Engine/EditorBlueprintResources/StandardMacros.DoOnce` true :!label _label
    (:`Completed`
      (if (not (and (and (`self.isSpawning`) (== (`self.GetSpawnedEnemyCount`) 0)) (`self.IsAnnihilationFinish`)))
        (`KismetSystemLibrary.Delay` (`self.ForceFinishSeonds`)) ; 一定時間待機で強制的に終了させる
      )
      (`KismetSystemLibrary.Delay` (`self.SurplusWaitSeconds`)) ; 終了後の待機時間
      ;[1 1 1] スポーン終了
      (`self.FinishSpawn`))))

(fn `UserConstructionScript`)