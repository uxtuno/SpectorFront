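; Test actor that ping-pongs sideways around its spawn point until it takes damage.
; Each Tick while alive, Move sweeps it along the mesh's right vector by speed and delta time, reversing direction once its distance from the start location reaches SwitchDistance.
; Any damage counts as death, stopping the movement and turning on physics simulation for the mesh.
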(event `self.ReceiveBeginPlay`
  (set `self.StartLocation` (`self.K2_GetActorLocation`))
  (set `self.IsLife` true))

(event `self.ReceiveTick`
  (params (DeltaSeconds :type "Float (single-precision)"))
  (if (`self.IsLife`)
    (`self.Move` DeltaSeconds)
    (if (>= (`KismetMathLibrary.VSize` (- (`self.StartLocation`) (`self.K2_GetActorLocation`))) (`self.SwitchDistance`))
      (set `self.IsMoveRight` (not (`self.IsMoveRight`))))))

(event `self.ReceiveAnyDamage`
  (params (Damage :type "Float (single-precision)") (DamageType :type "DamageType Object Reference") (InstigatedBy :type "Controller Object Reference") (DamageCauser :type "Actor Object Reference"))
  ;[1 1 1] 死亡
  (`PrimitiveComponent.SetSimulatePhysics` (`self.Mesh`) true)
  (set `self.IsLife` false))

(fn `Move`
  (params (A :type "Float (double-precision)"))
  (bind _returnvalue (`self.K2_GetActorLocation`))
  (bind _returnvalue_2 (* (`SceneComponent.GetRightVector` (`self.Mesh`)) (* A (`self.Spped`))))
  (if (`self.IsMoveRight`)
    (`self.K2_SetActorLocation` (+ _returnvalue _returnvalue_2) true)
    (else
      (`self.K2_SetActorLocation` (+ _returnvalue (* _returnvalue_2 -1)) true)))
  (return))

(fn `UserConstructionScript`)