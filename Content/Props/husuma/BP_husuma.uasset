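; Sliding fusuma door Blueprint that parts its CenterLeft and CenterRight panels.
; Timeline_0's Open track drives both panels' relative X in mirrored directions from a fixed offset.
; Actor overlap restarts the timeline from the start, while Tick also calls Play every frame, so opening does not depend on overlap.
; No closing or reverse logic exists.
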(event `self.ReceiveActorBeginOverlap`
  (params (OtherActor :type "Actor Object Reference"))
  (bind _centerright (`self.CenterRight`))
  (bind _centerleft (`self.CenterLeft`))
  (bind (_relativelocation_x _relativelocation_y _relativelocation_z) (`KismetMathLibrary.BreakVector` (`SceneComponent.RelativeLocation` _centerright)))
  (bind (_relativelocation_x_2 _relativelocation_y_2 _relativelocation_z_2) (`KismetMathLibrary.BreakVector` (`SceneComponent.RelativeLocation` _centerleft)))
  (bind (_direction _open) (`Timeline|Timeline_0` :!via `PlayFromStart` :!label _label)
    (:`Update`
      (bind _returnvalue (+ (* _open 180.0) 134.447754))
      (`SceneComponent.K2_SetRelativeLocation` _centerleft (`KismetMathLibrary.MakeVector` (* _returnvalue -1.0) _relativelocation_y_2 _relativelocation_z_2) false false)
      (`SceneComponent.K2_SetRelativeLocation` _centerright (`KismetMathLibrary.MakeVector` _returnvalue _relativelocation_y _relativelocation_z) false false))))

(event `self.ReceiveTick`
  (params (DeltaSeconds :type "Float (single-precision)"))
  (goto _label))

(fn `UserConstructionScript`)