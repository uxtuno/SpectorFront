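; Action phase actor that runs a series of enemy spawners during a level sequence, optionally pausing the sequence.
; BeginActionPhase starts the spawners one after another, each finish callback triggering the next, then opens a Tick gate.
; Tick waits until the last spawner's enemies are gone, unless ignorable, then delays.
; If the sequence stop flag is set, it then resumes playback and notifies the manager that the action ended.
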(event `self.ReceiveBeginPlay`
  (`parent.ReceiveBeginPlay`))

(event `self.ReceiveTick`
  (params (DeltaSeconds :type "Float (single-precision)"))
  (bind _currentspawner (`self.CurrentSpawner`))
  (`parent.ReceiveTick` DeltaSeconds)
  (`/Engine/EditorBlueprintResources/StandardMacros.Gate` true :!label _label ; 全てのスポーンが完了した後に処理を開始
    (:`Exit`
      (if (`self.IsIgnoreble`)
        (`KismetSystemLibrary.Delay` (`self.LateWaitSeconds`) :!label _label_2)
        (`self.ResumeSequencer` (`LevelSequenceActor.SequencePlayer` (stale `BeginActionPhase` Sequencer))) ; シーケンサーを再開
        (else
          ;[1 1 1] 敵が全滅するまで待機
          (if (!= _currentspawner null)
            (if (== (`self.GetSpawnedEnemyCount` _currentspawner) 0)
              (goto _label_2))))))))

(event `OnFinishSpawn`
  ;[1 1 1] 次のSpawnerを起動する
  (`self.ExecNextSpawner` (make `FinishSpawn` (delegate `OnFinishSpawn`)) :!label _label_3
    (:`Completed`
      (goto _label :!via `Open`))))

(event `BeginActionPhase`
  (params (ActionPhaseManager :type "/Game/Test/BluePrints/BP_ActionPhaseManager Object Reference") (Sequencer :type "LevelSequenceActor Object Reference") (ActorContainer :type "ActorContainer Object Reference"))
  ;[1 1 1] アクションフェーズ開始
  (set `self.AllActors` ActorContainer)
  (set `self.Manager` ActionPhaseManager)
  (`|ExecutionSequence`
    (:`then_0`
      (goto _label_3))
    (:`then_1`
      (if (`self.IsSequenceStop`)
        (`LevelSequencePlayer.Pause` (`LevelSequenceActor.SequencePlayer` Sequencer))))))

(fn `NextSpawn`)

(fn `ResumeSequencer`
  (params (NewParam :type "LevelSequencePlayer Object Reference"))
  (if (`self.IsSequenceStop`)
    (`LevelSequencePlayer.Play` NewParam)
    (`/Game/Test/BluePrints/BP_ActionPhaseManager.OnActionEnd` (`self.Manager`))))

(fn `UserConstructionScript`)