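; Enemy spawn controller that runs the spawners in SpawnerList one after another.
; Tick drives a DoOnce gate, which BeginSpawn resets to start the sequence after calling its parent implementation.
; Each pass calls Spawn on the current spawner with itself as argument and advances the index, and OnComplete reopens the gate for the next.
; Once the list is exhausted, it calls EndSpawn after a short delay.
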(event `self.ReceiveTick`
  (params (DeltaSeconds :type "Float (single-precision)"))
  (bind _spawnerindex (`self.SpawnerIndex`))
  (`/Engine/EditorBlueprintResources/StandardMacros.DoOnce` true :!label _label
    (:`Completed`
      (if (< _spawnerindex (`KismetArrayLibrary.Array_Length` (`self.spawnerList`)))
        (`EnemySpawner.Spawn` (`KismetArrayLibrary.Array_Get` (`self.spawnerList`) _spawnerindex) self)
        (`/Engine/EditorBlueprintResources/StandardMacros.IncrementInt` (`self.SpawnerIndex`))
        (else
          (`KismetSystemLibrary.Delay` 5.0)
          (`self.EndSpawn`))))))

(event `self.OnComplete`
  (goto _label :!via `Reset`))

(event `self.BeginSpawn`
  (params (completeEvent :type "Delegate (by ref)"))
  (`parent.BeginSpawn` completeEvent)
  (goto _label :!via `Reset`))

(fn `UserConstructionScript`)