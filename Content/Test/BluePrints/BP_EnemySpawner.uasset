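; Enemy spawner Blueprint that decides when a spawn sequence finishes, building on a parent spawner's begin-spawn logic.
; Begin spawn opens a Gate that Tick passes through every frame to check the end condition.
; All spawned enemies being gone while spawning, with IsKillAndForceFinish set, skips the forced-finish timeout; otherwise that Delay runs.
; Both paths then wait a surplus delay before calling FinishSpawn, and the Gate is never closed here.
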(event `self.OnBeginSpawn`
  (`parent.OnBeginSpawn`)
  (goto _label :!via `Open`))

(event `self.ReceiveTick`
  (params (DeltaSeconds :type "Float (single-precision)"))
  (`/Engine/EditorBlueprintResources/StandardMacros.Gate` true :!label _label ; スポーン開始時から処理を始める
    (:`Exit`
      (if (not (and (and (`self.isSpawing`) (== (`self.GetSpawnedEnemyCount`) 0)) (`self.IsKillAndForceFinish`)))
        (`KismetSystemLibrary.Delay` (`self.ForceFinishSeonds`)) ; 一定時間待機で強制的に終了させる
      )
      (`KismetSystemLibrary.Delay` (`self.SurplusWaitSeconds`)) ; 終了後の待機時間
      ;[1 1 1] スポーン終了
      (`self.FinishSpawn`))))

(fn `UserConstructionScript`)