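; Test actor that wraps a Spline component and exposes path queries by distance.
; GetCurrentLocation returns the world location at a given distance along the spline, though its Loop branch wraps the local LocalLength instead of the Length input.
; GetSplineLength returns the total length, and IsArrived reports whether a distance has reached the end.
; The event graph and construction script are empty.
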(fn `GetCurrentLocation`
  (params (Length :type "Float (double-precision)") (Loop :type Boolean))
  (returns (Location :type "Vector Structure"))
  (if Loop
    (set `self.LocalLength` (mod (`self.LocalLength`) (`SplineComponent.GetSplineLength` (`self.Spline`))))
    (else
      (set `self.LocalLength` Length)))
  (return (`SplineComponent.GetLocationAtDistanceAlongSpline` (`self.Spline`) (`self.LocalLength`) "World")))

(fn `GetSplineLength`
  (returns (Length :type "Float (double-precision)"))
  (return (`SplineComponent.GetSplineLength` (`self.Spline`))))

(fn `IsArrived`
  (params (Length :type "Float (double-precision)"))
  (returns (IsArrived :type Boolean))
  (return (>= Length (`SplineComponent.GetSplineLength` (`self.Spline`)))))

(fn `UserConstructionScript`)