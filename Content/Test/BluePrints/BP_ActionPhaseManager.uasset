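; BP_ActionPhaseManager is an actor that runs action phases from a list for a sequencer.
; BeginAction starts the phase at the current index, if it lies within the list, passing itself and the sequencer along.
; OnActionEnd forwards to CallEndActionPhase, and the construction script calls SetActorLocationAndRotation.
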(event `BeginAction`
  (params (Sequencer :type "LevelSequenceActor Object Reference"))
  (bind _currentactionphaseindex (`self.CurrentActionPhaseIndex`))
  (if (< _currentactionphaseindex (`KismetArrayLibrary.Array_Length` (`self.ActionPhaseList`)))
    (`/Game/Test/BluePrints/BP_ActionPhase.BeginActionPhase` (`KismetArrayLibrary.Array_Get` (`self.ActionPhaseList`) _currentactionphaseindex) self Sequencer)))

(event `OnActionEnd`
  (`self.EndActionPhase`))

(fn `UserConstructionScript`
  (`self.K2_SetActorLocationAndRotation` (0.0 0.0 0.0)))